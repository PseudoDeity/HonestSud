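; BP_Ammo_Pickup is a single-use ammo pickup that refills the first-person character's Ammo to 100.
; Overlapping the Ammo component refills a character that is not at exactly 100, then sets Consumed; otherwise it prints a debug message.
; ConsumedStateEvent then hides the Cube and disables its collision.
; Nothing here resets Consumed, so later overlaps only print "Ammo not ready yet!".
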(event OnComponentBeginOverlap(Ammo)
  (params (OverlappedComponent :type Primitive%20Component%20Object%20Reference) (OtherActor :type Actor%20Object%20Reference) (OtherComp :type Primitive%20Component%20Object%20Reference) (OtherBodyIndex :type Integer) (bFromSweep :type Boolean) (SweepResult :type Hit%20Result%20Structure%20%28by%20ref%29))
  (bind _asbp_first_person_character (Utilities|Casting|CastToBP_FirstPersonCharacter OtherActor))
  (Variables|Default|SetAs%20BP%20First%20Person%20Character _asbp_first_person_character)
  (if (Variables|Default|GetConsumed)
    (Development|PrintString "Ammo not ready yet!")
    (elif (== (Variables|/Game/FirstPerson/Blueprints/BP_FirstPersonCharacter.BP_FirstPersonCharacter_C|GetAmmo (Variables|Default|GetAs%20BP%20First%20Person%20Character)) 1e+02)
      (Development|PrintString "Ammo is Full")
      (else
        (Variables|/Game/FirstPerson/Blueprints/BP_FirstPersonCharacter.BP_FirstPersonCharacter_C|SetAmmo (Variables|Default|GetAs%20BP%20First%20Person%20Character) 1e+02)
        (Variables|Default|SetConsumed true)
        (CallFunction|ConsumedStateEvent)))))

(event Custom|ConsumedStateEvent
  (bind _cube (Variables|Default|GetCube))
  (if (Variables|Default|GetConsumed)
    (Development|PrintString "True")
    (Development|SetHiddeninGame _cube true false)
    (Collision|SetCollisionEnabled _cube "NoCollision")
    (else
      (Development|PrintString "False"))))

(fn ConstructionScript)