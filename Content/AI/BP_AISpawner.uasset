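; BP_AISpawner is an enemy spawner that holds a queue of enemy classes and spawns them at its own transform.
; A looping timer spawns the next queued enemy, and adding to the queue spawns immediately if no BP_AI overlaps its Sphere.
; It binds to each enemy's destroyed event and has a handler that reports defeats to BP_FirstPersonGameMode.
; Tick sets IsOn from player overlap with ActiveBox, though spawning here ignores that flag.
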(event Custom|TryToSpawnEnemy
  (CallFunction|SpawnEnemy))

(event Custom|OnEnemyDefeated
  (bind _asbp_first_person_game_mode (Utilities|Casting|CastToBP_FirstPersonGameMode (Game|GetGameMode)))
  (Default|OnEnemyDefeated _asbp_first_person_game_mode))

(event EventBeginPlay
  (Utilities|FlowControl|Sequence
    (:then_0
      (Utilities|FlowControl|Delay 0.1))
    (:then_1
      (Utilities|Time|SetTimerbyEvent (delegate Custom|TryToSpawnEnemy) 3.2 true))))

(event EventTick
  (params (DeltaSeconds :type Float%20%28single-precision%29))
  (if (Collision|IsOverlappingActor (Variables|Default|GetActiveBox) (Game|GetPlayerCharacter 0) :!class /Script/Engine.PrimitiveComponent)
    (Variables|Default|SetIsOn? true)
    (else
      (Variables|Default|SetIsOn? false))))

(fn ConstructionScript)

(fn SpawnEnemy
  (if (Utilities|Array|IsValidIndex (Variables|Default|GetEnemyQueue))
    (bind _returnvalue (Game|SpawnActorfromClass (Utilities|Array|Get(acopy) (Variables|Default|GetEnemyQueue)) (Transformation|GetActorTransform) "Undefined" "MultiplyWithRoot" 0 0))
    (EventDispatchers|BindEventtoOnEnemyDestroyed _returnvalue (EventDispatchers|CreateEvent :!event Custom|OnEnemyDefeated))
    (Utilities|Array|RemoveIndex (Variables|Default|GetEnemyQueue))
    (return true)
    (else
      (return false))))

(fn AddEnemytoQueue
  (params (EnemyClass :type BP%20AI%20Class%20Reference%20%28by%20ref%29))
  (Utilities|Array|Add (Variables|Default|GetEnemyQueue) EnemyClass)
  (if (not (Utilities|Array|IsValidIndex (Collision|GetOverlappingActors (Variables|Default|GetSphere) "/Game/AI/BP_AI.BP_AI_C" :!class /Script/Engine.PrimitiveComponent)))
    (CallFunction|SpawnEnemy)))